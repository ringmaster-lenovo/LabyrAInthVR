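; BP_Enemy is an enemy pawn in the VRCore content that chases pawns it sees.
; Its PawnSensing component's OnSeePawn event issues an AI MoveTo with the seen pawn as the target actor, with no filtering of which pawn that is.
; A GetSpeed helper returns the CharacterMovement velocity length.
; An unconnected AI MoveTo toward a point offset along world X never runs.
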(event `self.ReceiveBeginPlay`)

(event `self.PawnSensing.OnSeePawn`
  (params (Pawn :type "Pawn Object Reference"))
  (`|AIMoveTo` self (0.0 0.0 0.0) Pawn))

(event `self.ReceiveTick`
  (params (DeltaSeconds :type "Float (single-precision)")))

(fn `GetSpeed`
  (returns (Speed :type "Float (double-precision)"))
  (bind _charactermovement (`self.CharacterMovement`))
  (`/Engine/EditorBlueprintResources/StandardMacros.IsValid` _charactermovement
    (:`Is Valid`
      (return (`KismetMathLibrary.VSize` (`MovementComponent.Velocity` _charactermovement))))))

(fn `UserConstructionScript`)