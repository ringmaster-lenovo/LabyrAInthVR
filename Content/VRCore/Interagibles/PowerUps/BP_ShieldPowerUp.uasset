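; Shield power-up pickup, an interactable in the VR game that is collected on overlap.
; BeginPlay sets the shield collect sound and binds its own begin and end overlap events.
; Begin overlap calls OnCollect with Stats and StatsChanger and spawns a Niagara coin burst at the root's transform.
; The actor destroys itself only when the overlap ends, and neither handler filters the overlapping actor.
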(event `self.ReceiveBeginPlay`
  (set `self.CollectSound` "/Game/VRCore/Interagibles/Sound/Shield.Shield")
  (add `self.OnActorBeginOverlap` (delegate `BeginEvent`))
  (add `self.OnActorEndOverlap` (delegate `EndEvent`)))

(event `BeginEvent` :!signature `self.OnActorBeginOverlap`
  (params (OverlappedActor :type "Actor Object Reference") (OtherActor :type "Actor Object Reference"))
  (bind (_returnvalue_location _returnvalue_rotation _returnvalue_scale) (`KismetMathLibrary.BreakTransform` (`SceneComponent.GetRelativeTransform` (`self.DefaultSceneRoot`))))
  (`self.OnCollect` (`self.Stats`) (`self.StatsChanger`))
  (`NiagaraFunctionLibrary.SpawnSystemAtLocation` "/Game/sA_PickupSet_1/Fx/NiagaraSystems/NS_CoinBurst.NS_CoinBurst" _returnvalue_location _returnvalue_rotation _returnvalue_scale))

(event `EndEvent` :!signature `self.OnActorEndOverlap`
  (params (OverlappedActor :type "Actor Object Reference") (OtherActor :type "Actor Object Reference"))
  (`self.K2_DestroyActor`))

(fn `UserConstructionScript`)