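; BP_MusicController is an actor that plays background and combat music, with separate ambience for the lobby.
; StartAmbienceMusic fades out a valid current track, then ChooseBackgroundMusic adds the lobby track or one of three random tracks to fade in.
; An audio-finished binding repeats the selection for continuous playback.
; Combat music plays on its own component, SetMusicVolume only stores the value, and StartFinalResultMusic is empty.
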(event `self.StartAmbienceMusic`
  (params (bIsInLobby :type Boolean))
  (bind _ambient (`self.Ambient`))
  (if (`KismetSystemLibrary.IsValid` _ambient)
    (remove `AudioComponent.OnAudioFinished` _ambient (delegate `OnAudioFinished_Event`))
    (`AudioComponent.FadeOut` _ambient 2.0 0.0 "Linear")
    (bind _output_get (set `self.bInLobby` bIsInLobby))
    (bind _sound (`self.ChooseBackgroundMusic` _output_get :!label _label))
    (`KismetSystemLibrary.PrintString` (`KismetSystemLibrary.GetDisplayName` _sound))
    (bind _output_get_2 (set `self.Ambient` _sound))
    (if (`KismetSystemLibrary.IsValid` _output_get_2)
      (`AudioComponent.FadeIn` _output_get_2 2.0 1.0 0.0 "Linear")
      (add `AudioComponent.OnAudioFinished` _output_get_2 (delegate `OnAudioFinished_Event`)))))

(event `self.ReceiveBeginPlay`)

(event `OnAudioFinished_Event`
  (remove `AudioComponent.OnAudioFinished` (stale `self.StartAmbienceMusic` _output_get_2) (delegate `OnAudioFinished_Event`))
  (goto _label))

(event `self.StartFinalResultMusic`
  (params (bHasWon :type Boolean)))

(event `self.StartCombatMusic`
  (bind _returnvalue (`AddComponent|NODE_AddAudioComponent-4`))
  (bind _output_get (set `self.Combat` _returnvalue))
  (`AudioComponent.Play` _output_get 0.0)
  (set `self.bIsMusicPlaying` true))

(event `self.SetMusicVolume`
  (params (Volume :type "Float (single-precision)"))
  (set `self.MusicVolume` Volume))

(fn `ChooseBackgroundMusic`
  (params (InLobby :type Boolean))
  (returns (Sound :type "AudioComponent Object Reference"))
  (if InLobby
    (bind _returnvalue (`AddComponent|NODE_AddAudioComponent-9`))
    (set `self.MusicChosen` _returnvalue)
    (else
      (switch `int` (`KismetMathLibrary.RandomInteger` 3)
        (:`Default`
          (bind _returnvalue_2 (`AddComponent|NODE_AddAudioComponent-7` :!label _label))
          (set `self.MusicChosen` _returnvalue_2))
        (:`0`
          (goto _label))
        (:`1`
          (bind _returnvalue_3 (`AddComponent|NODE_AddAudioComponent-8`))
          (set `self.MusicChosen` _returnvalue_3))
        (:`2`
          (bind _returnvalue_4 (`AddComponent|NODE_AddAudioComponent-14`))
          (set `self.MusicChosen` _returnvalue_4)))))
  (return (`self.MusicChosen`)))

(fn `UserConstructionScript`)