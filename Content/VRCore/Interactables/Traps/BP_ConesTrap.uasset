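; BP_ConesTrap is a one-shot trap actor that thrusts cones up after something overlaps its TriggerArea.
; The overlap plays an alert sound and, after a delay, plays a second sound while MoveComponentTo quickly moves the cones to their raised position.
; It then calls ApplyDamage, currently an empty stub, lowers the cones more slowly and destroys itself.
; The overlap has no actor filter or re-entry guard.
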(event `self.ReceiveBeginPlay`)

(event `self.TriggerArea.OnComponentBeginOverlap`
  (params (OverlappedComponent :type "PrimitiveComponent Object Reference") (OtherActor :type "Actor Object Reference") (OtherComp :type "PrimitiveComponent Object Reference") (OtherBodyIndex :type Integer) (bFromSweep :type Boolean) (SweepResult :type "HitResult Structure (by ref)"))
  (`GameplayStatics.PlaySoundAtLocation` (`self.AlertSound`) (`SceneComponent.K2_GetComponentLocation` (`self.DefaultSceneRoot`)) (struct) 1.0 1.0 0.0 null null null null)
  (`KismetSystemLibrary.Delay` 4.0)
  (`GameplayStatics.PlaySoundAtLocation` (`self.CollectSound`) (`SceneComponent.K2_GetComponentLocation` (`self.DefaultSceneRoot`)) (struct) 1.0 1.0 0.0 null null null null)
  (`KismetSystemLibrary.MoveComponentTo` (`self.cones`) (0.0 0.0 0.0) (struct) false false 0.1)
  (`self.ApplyDamage`)
  (`KismetSystemLibrary.MoveComponentTo` (`self.cones`) (0.0 0.0 -150.0) (struct) false false 1.0)
  (`self.K2_DestroyActor`))

(fn `ApplyDamage`)

(fn `UserConstructionScript`)