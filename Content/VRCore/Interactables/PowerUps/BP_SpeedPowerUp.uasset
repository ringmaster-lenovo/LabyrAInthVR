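; Speed power-up pickup for the VR game, collected when an actor parented to the MainCharacter overlaps it.
; BeginPlay binds its own begin and end overlap events, both casting the other actor's parent to MainCharacter.
; Begin overlap passes Stats and StatsChanger to OnCollect and spawns the NS_Energy_2 effect using the root's relative transform.
; The pickup destroys itself when that overlap ends, not on collection.
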(event `self.ReceiveBeginPlay`
  (add `self.OnActorBeginOverlap` (delegate `BeginEvent`))
  (add `self.OnActorEndOverlap` (delegate `EndEvent`)))

(event `BeginEvent` :!signature `self.OnActorBeginOverlap`
  (params (OverlappedActor :type "Actor Object Reference") (OtherActor :type "Actor Object Reference"))
  (bind (_returnvalue_location _returnvalue_rotation _returnvalue_scale) (`KismetMathLibrary.BreakTransform` (`SceneComponent.GetRelativeTransform` (`self.DefaultSceneRoot`))))
  (cast `MainCharacter` (`self.GetParentActor` OtherActor))
  (`self.OnCollect` (`self.Stats`) (`self.StatsChanger`))
  (`NiagaraFunctionLibrary.SpawnSystemAtLocation` "/Game/sA_PickupSet_1/Fx/NiagaraSystems/NS_Energy_2.NS_Energy_2" _returnvalue_location _returnvalue_rotation _returnvalue_scale))

(event `EndEvent` :!signature `self.OnActorEndOverlap`
  (params (OverlappedActor :type "Actor Object Reference") (OtherActor :type "Actor Object Reference"))
  (cast `MainCharacter` (`self.GetParentActor` OtherActor))
  (`self.K2_DestroyActor`))

(fn `UserConstructionScript`)