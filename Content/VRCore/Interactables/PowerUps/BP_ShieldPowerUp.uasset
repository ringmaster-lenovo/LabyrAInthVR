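; BP_ShieldPowerUp is a collectible shield power-up that switches on the main character's armor stat when touched.
; Its Collision component's begin-overlap event filters for a MainCharacter with a valid PlayerStats, then enables the Armor boolean stat through ChangeStatBool.
; On pickup it spawns a shield effect system and plays a collect sound at its root's location, then destroys itself.
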(event `self.ReceiveBeginPlay`)

(event `self.Collision.OnComponentBeginOverlap`
  (params (OverlappedComponent :type "PrimitiveComponent Object Reference") (OtherActor :type "Actor Object Reference") (OtherComp :type "PrimitiveComponent Object Reference") (OtherBodyIndex :type Integer) (bFromSweep :type Boolean) (SweepResult :type "HitResult Structure (by ref)"))
  (bind (_returnvalue_location _returnvalue_rotation) (`KismetMathLibrary.BreakTransform` (`SceneComponent.K2_GetComponentToWorld` (`self.DefaultSceneRoot`))))
  (if (and (`GameplayStatics.ObjectIsA` OtherActor "/Script/LabyrAInthVR.MainCharacter") (`KismetSystemLibrary.IsValid` OtherActor))
    (bind _asmain_character (cast `MainCharacter` OtherActor))
    (bind _playerstats (`MainCharacter.PlayerStats` _asmain_character))
    (if (`KismetSystemLibrary.IsValid` _playerstats)
      (`PlayerStatistics.ChangeStatBool` _playerstats "Esm_Armor" true)
      (`NiagaraFunctionLibrary.SpawnSystemAtLocation` "/Game/sA_PickupSet_1/Fx/NiagaraSystems/NS_Shield_4.NS_Shield_4" _returnvalue_location _returnvalue_rotation)
      (`GameplayStatics.PlaySoundAtLocation` (`self.CollectSound`) _returnvalue_location (struct) 1.0 1.0 0.0 null null null null)
      (`self.K2_DestroyActor`))))

(fn `UserConstructionScript`)