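; BP_StarPowerUp is a collectible star power-up that triggers the SpawnManager's frozen star effect when the MainCharacter touches it.
; On Collision overlap, it looks up the SpawnManager by class, removes itself from that manager's list and calls TriggerFrozenStar.
; It then spawns an effect and plays the collect sound at its root before destroying itself.
; Without a valid SpawnManager, the pickup does nothing.
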(event `self.ReceiveBeginPlay`)

(event `self.Collision.OnComponentBeginOverlap`
  (params (OverlappedComponent :type "PrimitiveComponent Object Reference") (OtherActor :type "Actor Object Reference") (OtherComp :type "PrimitiveComponent Object Reference") (OtherBodyIndex :type Integer) (bFromSweep :type Boolean) (SweepResult :type "HitResult Structure (by ref)"))
  (bind (_returnvalue_location _returnvalue_rotation) (`KismetMathLibrary.BreakTransform` (`SceneComponent.K2_GetComponentToWorld` (`self.DefaultSceneRoot`))))
  (if (and (`KismetSystemLibrary.IsValid` OtherActor) (`GameplayStatics.ObjectIsA` OtherActor "/Script/LabyrAInthVR.MainCharacter"))
    (bind _returnvalue (`GameplayStatics.GetActorOfClass` "/Script/LabyrAInthVR.SpawnManager"))
    (`/Engine/EditorBlueprintResources/StandardMacros.IsValid` _returnvalue
      (:`Is Valid`
        (`SpawnManager.RemoveFromList` _returnvalue self)
        (`SpawnManager.TriggerFrozenStar` _returnvalue)
        (`NiagaraFunctionLibrary.SpawnSystemAtLocation` null _returnvalue_location _returnvalue_rotation)
        (`GameplayStatics.PlaySoundAtLocation` (`self.CollectSound`) _returnvalue_location (struct) 1.0 1.0 0.0 null null null null)
        (`self.K2_DestroyActor`)))))

(fn `Logic`)

(fn `UserConstructionScript`)